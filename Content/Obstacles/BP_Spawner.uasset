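; BP_Spawner is an obstacle spawner that keeps producing vehicles at its own location and rotation.
; On BeginPlay it randomly picks one vehicle class (bus, truck or sportscar), a spawn interval and a population limit, then starts a looping timer.
; Each tick of the timer spawns only while under the limit and the SpawnClearance area holds no BP_Vehicle.
; Destroyed-event bindings decrement the live count to free slots.
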(event `self.ReceiveBeginPlay`
  (`|ExecutionSequence`
    (:`then_0`
      (`self.RandomizeVehicle`))
    (:`then_1`
      (`self.RandomizeSpawnRate`))
    (:`then_2`
      (`self.RandomizeSpawnLimit`))
    (:`then_3`
      (`KismetSystemLibrary.K2_SetTimerDelegate` (delegate `TrySpawn`) (`self.SpawnRate`) true))))

(event `TrySpawn`
  (if (< (`self.CurrentCount`) (`self.SpawnLimit`))
    (if (== (`KismetArrayLibrary.Array_Length` (`PrimitiveComponent.GetOverlappingActors` (`self.SpawnClearance`) "/Game/Obstacles/BP_Vehicle.BP_Vehicle_C")) 0)
      (bind _returnvalue (`|SpawnActorFromClass` (`self.ActorToSpawn`) (`KismetMathLibrary.MakeTransform` (`self.K2_GetActorLocation`) (`self.K2_GetActorRotation`)) "DontSpawnIfColliding" "MultiplyWithRoot" null null))
      (`/Engine/EditorBlueprintResources/StandardMacros.IncrementInt` (`self.CurrentCount`)
        (:`  `
          (add `self.OnDestroyed` _returnvalue (delegate `RemoveCount`))
          (`KismetSystemLibrary.PrintString` (`KismetStringLibrary.Concat_StrStr` "New Object spawned:  " (`KismetSystemLibrary.GetDisplayName` _returnvalue))))))))

(event `RemoveCount` :!signature `self.OnDestroyed`
  (params (DestroyedActor :type "Actor Object Reference"))
  (`/Engine/EditorBlueprintResources/StandardMacros.DecrementInt` (`self.CurrentCount`)
    (:`  `
      (`KismetSystemLibrary.PrintString` "Spawnable Destroyed"))))

(fn `RandomizeSpawnLimit`
  (set `self.SpawnLimit` (`KismetMathLibrary.RandomIntegerInRange` 3 7)))

(fn `RandomizeSpawnRate`
  (set `self.SpawnRate` (`KismetMathLibrary.RandomFloatInRange` 0.5 2.5)))

(fn `RandomizeVehicle`
  (set `self.ActorToSpawn` (select `int` (`KismetMathLibrary.RandomIntegerInRange` 0 2) :`0` "/Game/Obstacles/BP_Bus.BP_Bus_C" :`1` "/Game/Obstacles/BP_Truck.BP_Truck_C" :`2` "/Game/Obstacles/BP_Sportscar.BP_Sportscar_C" :!type "/Game/Obstacles/BP_Vehicle Class Reference")))

(fn `UserConstructionScript`)