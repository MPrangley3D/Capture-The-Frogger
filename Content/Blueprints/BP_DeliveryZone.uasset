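; BP_DeliveryZone is the flag drop-off zone in Capture the Frog that completes the current level.
; When a BP_Flag overlaps its box, a one-shot gate hides the flag's mesh, reveals the zone's victory flag and plays a stinger.
; After a short delay it increments CurrentLevel on the game instance and opens TopDownMap, so level progress carries across the map load.
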(event `self.Box.OnComponentBeginOverlap`
  (params (OverlappedComponent :type "PrimitiveComponent Object Reference") (OtherActor :type "Actor Object Reference") (OtherComp :type "PrimitiveComponent Object Reference") (OtherBodyIndex :type Integer) (bFromSweep :type Boolean) (SweepResult :type "HitResult Structure (by ref)"))
  (bind _asbp_flag (cast `/Game/Blueprints/BP_Flag` OtherActor))
  (`/Engine/EditorBlueprintResources/StandardMacros.DoOnce` false
    (:`Completed`
      (`SceneComponent.SetHiddenInGame` (`/Game/Blueprints/BP_Flag.FlagMesh` _asbp_flag) true false)
      (`SceneComponent.SetHiddenInGame` (`self.VictoryFlag`) false false)
      (`GameplayStatics.PlaySound2D` "/Game/Retro_8Bit_Sounds/Music/Wavs/retro__musical_stinger_03.retro__musical_stinger_03" 1.0 1.0 0.0 null null)
      (`KismetSystemLibrary.Delay` 3.0)
      (bind _asgi_capture_the_frog (cast `/Game/Blueprints/GI_CaptureTheFrog` (`GameplayStatics.GetGameInstance`)))
      (`/Engine/EditorBlueprintResources/StandardMacros.IncrementInt` (`/Game/Blueprints/GI_CaptureTheFrog.CurrentLevel` _asgi_capture_the_frog)
        (:`  `
          (`GameplayStatics.OpenLevel` "TopDownMap"))))))

(fn `UserConstructionScript`)